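; Toon Tanks game mode Blueprint that handles the UI for the start and end of a match.
; StartGame clears existing widgets, then adds the start game and gameplay widgets to the viewport for the Toon Tanks player controller.
; GameOver adds the end game widget and sets its display text to a win or loss message based on the WonGame flag.
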(event EventBeginPlay)

(event EventStartGame
  (Viewport|RemoveAllWidgets)
  (bind _returnvalue (UserInterface|CreateWidget "/Game/Blueprints/Widgets/WBP_StartGameWidget.WBP_StartGameWidget_C" (Variables|Default|GetToonTanksPlayerController)))
  (UserInterface|Viewport|AddtoViewport _returnvalue 0)
  (bind _returnvalue_2 (UserInterface|CreateWidget "/Game/Blueprints/Widgets/WBP_GameplayWidget.WBP_GameplayWidget_C" (Variables|Default|GetToonTanksPlayerController)))
  (UserInterface|Viewport|AddtoViewport _returnvalue_2 0))

(event EventGameOver
  (params (WonGame :type Boolean))
  (bind _returnvalue (UserInterface|CreateWidget "/Game/Blueprints/Widgets/WBP_EndGameWidget.WBP_EndGameWidget_C" (Variables|Default|GetToonTanksPlayerController)))
  (UserInterface|Viewport|AddtoViewport _returnvalue 0)
  (Rendering|Components|TextRender|SetText (Variables|/Game/Blueprints/Widgets/WBP_EndGameWidget.WBP_EndGameWidget_C|GetDisplayText _returnvalue) (select WonGame "You Win!" "Game Over!")))

(fn ConstructionScript)